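; BP_PollutionVolume is an overlap volume that turns the number of actors inside it into a global pollution value for leaf colour.
; Begin and end overlap events add and remove actors in the Trees array, with no class filtering.
; Every tick it writes that count divided by 100, unclamped, to the Pollution scalar in the MPC_LeafColour material parameter collection.
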(event Collision|EventActorBeginOverlap
  (params (OtherActor :type Actor%20Object%20Reference))
  (Utilities|Array|Add (Variables|Default|GetTrees) OtherActor))

(event Collision|EventActorEndOverlap
  (params (OtherActor :type Actor%20Object%20Reference))
  (Utilities|Array|RemoveItem (Variables|Default|GetTrees) OtherActor))

(event EventTick
  (params (DeltaSeconds :type Float%20%28single-precision%29))
  (Rendering|Material|SetScalarParameterValue "/Game/Environment/MPC_LeafColour.MPC_LeafColour" "Pollution" (/ (Math|Conversions|ToFloat(Integer) (Utilities|Array|Length (Variables|Default|GetTrees))) 1e+02) :!class /Script/Engine.KismetMaterialLibrary))

(fn ConstructionScript)