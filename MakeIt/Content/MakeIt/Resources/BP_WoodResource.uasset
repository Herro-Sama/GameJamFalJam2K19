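; Harvestable wood resource tree that starts with a randomized amount of wood and changes to a chopped state once harvested.
; A looping timer polls the harvested flag and runs the cut sequence once.
; The cut shrinks the tree, swaps its mesh, removes grass and trunk collision, and reveals a physics-simulated chopped piece.
; After delays, the box component is destroyed and the loose piece is hidden.
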(event Custom|CheckIfCut
  (bind _choppedtree (Variables|Default|GetChoppedTree))
  (bind _tree (Variables|Default|GetTree))
  (if (Variables|Default|GetHasBeenHarvested)
    (Utilities|FlowControl|DoOnce false
      (:Completed
        (Transformation|SetWorldScale3D _tree "0.500000,0.500000,0.500000")
        (Components|StaticMesh|SetStaticMesh _tree "/Game/Environment/ChoppedTree_pCylinder3.ChoppedTree_pCylinder3")
        (Components|DestroyComponent (Variables|Default|GetGrassCollision))
        (Rendering|SetVisibility _choppedtree true false)
        (Physics|SetSimulatePhysics _choppedtree true)
        (Utilities|FlowControl|Delay 6.0)
        (Components|DestroyComponent (Variables|Default|GetBox))
        (Utilities|FlowControl|Delay 1.0)
        (Rendering|SetVisibility (Variables|Default|GetChoppedTree) false false)))))

(event EventBeginPlay
  (Variables|Default|SetResourceType 0)
  (Variables|Default|SetResourceAmount (Math|Random|RandomIntegerinRange 20 80))
  (Utilities|Time|SetTimerbyEvent (delegate Custom|CheckIfCut) 0.2 true))

(fn ConstructionScript)